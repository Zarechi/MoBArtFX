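; BP_MetricsTimer is a metrics gym stopwatch that times an actor travelling between a starting box and an ending box.
; Overlapping the start box stores the actor and starts a long looping timer with an empty event, used only for its elapsed time.
; When that same actor overlaps the end box, a result text shows time and average speed over an assumed 10 m gap, then the timer is cleared.
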(event OnComponentBeginOverlap(StartingBox)
  (params (OverlappedComponent :type Primitive%20Component%20Object%20Reference) (OtherActor :type Actor%20Object%20Reference) (OtherComp :type Primitive%20Component%20Object%20Reference) (OtherBodyIndex :type Integer) (bFromSweep :type Boolean) (SweepResult :type Hit%20Result%20Structure%20%28by%20ref%29))
  (Variables|Default|SetMeasuringActor OtherActor)
  (bind _returnvalue (Utilities|Time|SetTimerbyEvent (delegate Custom|EmptyEvent) 5e+02 true))
  (Variables|Default|SetTimerHandle _returnvalue))

(event OnComponentBeginOverlap(EndingBox)
  (params (OverlappedComponent :type Primitive%20Component%20Object%20Reference) (OtherActor :type Actor%20Object%20Reference) (OtherComp :type Primitive%20Component%20Object%20Reference) (OtherBodyIndex :type Integer) (bFromSweep :type Boolean) (SweepResult :type Hit%20Result%20Structure%20%28by%20ref%29))
  (bind _timerhandle (Variables|Default|GetTimerHandle))
  (bind _returnvalue (Class|KismetSystemLibrary|GetTimerElapsedTimeHandle _timerhandle))
  (bind _measuringactor (Variables|Default|GetMeasuringActor)
    (:then
      (if (== _measuringactor OtherActor)
        (Rendering|Components|TextRender|SetText (Variables|Default|GetResultScreen) (Utilities|Text|FormatText "Current Timer: {Timer}s 
Average Speed: {Speed}cm/s" (Utilities|Text|ToText(Float) _returnvalue "HalfToEven" false true 2 3 3) (Utilities|Text|ToText(Float) (/ 1e+03 _returnvalue) "HalfToEven" false true 1 5 2 2)))
        (Utilities|Time|ClearandInvalidateTimerbyHandle (Variables|Default|GetTimerHandle))))
    (:else)))

(event Custom|EmptyEvent)

(fn ConstructionScript)