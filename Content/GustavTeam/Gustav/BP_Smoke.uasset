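; BP_Smoke is a timed damage-zone actor, named as smoke, that hurts actors inside its Box and destroys itself after ten seconds.
; Box overlap events add and remove actors in an array, which is cleared just before destruction.
; Tick runs through a Delay, which throttles it to apply damage to every tracked actor roughly every half second.
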(event OnComponentBeginOverlap(Box)
  (params (OverlappedComponent :type Primitive%20Component%20Object%20Reference) (OtherActor :type Actor%20Object%20Reference) (OtherComp :type Primitive%20Component%20Object%20Reference) (OtherBodyIndex :type Integer) (bFromSweep :type Boolean) (SweepResult :type Hit%20Result%20Structure%20%28by%20ref%29))
  (Utilities|Array|AddUnique (Variables|Default|GetOther%20Actor) OtherActor))

(event OnComponentEndOverlap(Box)
  (params (OverlappedComponent :type Primitive%20Component%20Object%20Reference) (OtherActor :type Actor%20Object%20Reference) (OtherComp :type Primitive%20Component%20Object%20Reference) (OtherBodyIndex :type Integer))
  (Utilities|Array|RemoveItem (Variables|Default|GetOther%20Actor) OtherActor))

(event EventTick
  (params (DeltaSeconds :type Float%20%28single-precision%29))
  (Utilities|FlowControl|Delay 0.5)
  (for _array_element (Variables|Default|GetOther%20Actor)
    (Game|Damage|ApplyDamage _array_element 15.0 0 0)))

(event EventBeginPlay
  (Utilities|FlowControl|Delay 1e+01)
  (Utilities|Array|Clear (Variables|Default|GetOther%20Actor))
  (Actor|DestroyActor))

(fn ConstructionScript)