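; BP_PC_MoBArtFX is a player controller that stores the current gameplay state and exposes a getter and setter for it.
; It prints the state name on begin play.
; A debug key on P cycles the state through the enum, wrapping back to the first value, and prints the new state each time.
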(event EventSetGameplayState
  (params (GameplayState :type E_GameplayState%20Enum :default "NewEnumerator0"))
  (Variables|Default|SetGameplay%20State GameplayState))

(event EventBeginPlay
  (|CallParentFunction)
  (Development|PrintString (Utilities|String|EnumtoString (stale Input|KeyboardEvents|DebugKeyP _output_get))))

(event Input|KeyboardEvents|DebugKeyP
  (params (Key :type Key%20Structure :default "None") (ActionValue :type Input%20Action%20Value%20Structure))
  (:Pressed
    (bind _result (Math|Integer|IncrementInt (Math|Conversions|ToInteger(Byte) (Variables|Default|GetGameplay%20State)))
      (:%20%20
        (bind _output_get (Variables|Default|SetGameplay%20State (Utilities|Enum|ByteToEnumE_GameplayState (Math|Conversions|ToByte(Integer) (Math|Integer|SelectInt 0 _result (> _result 4))))))
        (Development|PrintString (Utilities|String|EnumtoString _output_get))))))

(fn ConstructionScript)

(fn GetGameplayState
  (return (Variables|Default|GetGameplay%20State)))