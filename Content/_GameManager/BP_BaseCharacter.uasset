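; BP_BaseCharacter is a base character Blueprint that handles health, damage and auto-attack bookkeeping through player data objects.
; On BeginPlay it constructs a debug player info instance from a data asset and fills its health to maximum, for testing.
; Damage lowers current health, clamped at zero, and calls Death when it reaches zero.
; AutoAttack extends the parent's attack by starting a data-driven cooldown and decrementing ammo.
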(event EventBeginPlay
  (|CallParentFunction)
  ;[1 0.8047 0] For Debugging and Testing. DataAsset informations are used to create DataAsset Instances
  (bind _debugplayerinfosasset (Variables|Default|GetDebugPlayerInfosAsset)
    (:then
      (bind _returnvalue (Game|ConstructObjectfromClass (Utilities|ResolveSoftReference _debugplayerinfosasset)))
      (Utilities|IsValid _returnvalue
        (:Is%20Valid
          (bind _output_get (Variables|Default|SetDebugPlayerInfos _returnvalue))
          (Variables|/Script/MoBArtFX.PlayerInfos|SetCurrentHealth _output_get (Variables|/Script/MoBArtFX.PlayerInfos|GetMaxHealth _output_get)))))
    (:else)))

(event EventAutoAttack
  (bind _returnvalue (Class|BaseCharacter|GetPlayerDatas))
  (|CallParentFunction)
  (Utilities|Cooldown (Variables|/Script/MoBArtFX.PlayerInfos|GetAutoAttack_CD _returnvalue) -1)
  (Math|Integer|DecrementInt (Variables|/Script/MoBArtFX.PlayerInfos|GetCurrentAmmo _returnvalue)))

(event Game|Damage|EventAnyDamage
  (params (Damage :type Float%20%28single-precision%29) (DamageType :type Damage%20Type%20Object%20Reference) (InstigatedBy :type Controller%20Object%20Reference) (DamageCauser :type Actor%20Object%20Reference))
  (bind _returnvalue (Class|BaseCharacter|GetPlayerDatas))
  (Utilities|IsValid _returnvalue
    (:Is%20Valid
      (bind _output_get (Variables|/Script/MoBArtFX.PlayerInfos|SetCurrentHealth _returnvalue (Math|Integer|Max(Integer) (Math|Float|Truncate (- (Variables|/Script/MoBArtFX.PlayerInfos|GetCurrentHealth _returnvalue) Damage)))))
      (if (== _output_get 0)
        (Class|BaseCharacter|Death)))))

(fn ConstructionScript)