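; BP_MeleeHit is a short-lived melee hit actor for the Cramptix auto attack.
; BeginPlay sets its lifespan from the auto-attack cooldown in PlayerData, which SetPlayerData supplies, and Tick counts it down until the actor destroys itself.
; When HitCapsule overlaps an actor of exactly the BP_Dummy class, it destroys both that dummy and itself.
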(event OnComponentBeginOverlap(HitCapsule)
  (params (OverlappedComponent :type Primitive%20Component%20Object%20Reference) (OtherActor :type Actor%20Object%20Reference) (OtherComp :type Primitive%20Component%20Object%20Reference) (OtherBodyIndex :type Integer) (bFromSweep :type Boolean) (SweepResult :type Hit%20Result%20Structure%20%28by%20ref%29))
  (if (== (Utilities|GetClass OtherActor) "/Game/Characters/Dummy/BP_Dummy.BP_Dummy_C")
    (Actor|DestroyActor OtherActor)
    (Actor|DestroyActor)))

(event EventBeginPlay
  (Variables|Default|SetcurrentLifeSpan (Variables|/Script/MoBArtFX.PlayerInfos|GetAutoAttack_CD (Variables|Default|GetplayerData))))

(event EventTick
  (params (DeltaSeconds :type Float%20%28single-precision%29))
  (bind _output_get (Variables|Default|SetcurrentLifeSpan (- (Variables|Default|GetcurrentLifeSpan) DeltaSeconds)))
  (if (< _output_get 0.0)
    (Actor|DestroyActor)))

(fn ConstructionScript)

(fn SetPlayerData
  (params (PlayerData :type Player%20Infos%20Object%20Reference))
  (Variables|Default|SetplayerData PlayerData))