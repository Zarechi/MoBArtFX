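; BP_Javlin is a thrown spell projectile in the Cramptix folder that repositions player 0 on impact.
; Its Cube gets a forward physics impulse on BeginPlay, and Tick destroys the actor once its lifespan expires.
; Hitting a BP_Dummy instantly moves player and dummy toward each other, just short of their midpoint.
; Any other hit moves the player to the impact point; both outcomes print debug text and destroy the javelin.
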(event OnComponentHit(Cube)
  (params (HitComponent :type Primitive%20Component%20Object%20Reference) (OtherActor :type Actor%20Object%20Reference) (OtherComp :type Primitive%20Component%20Object%20Reference) (NormalImpulse :type Vector :default "0, 0, 0") (Hit :type Hit%20Result%20Structure%20%28by%20ref%29))
  (CallFunction|JavlinHitting OtherActor (.ImpactPoint (Collision|BreakHitResult Hit))))

(event EventBeginPlay
  (bind _cube (Variables|Default|GetCube))
  (Physics|AddImpulse _cube (* (Math|Vector|GetForwardVector (Transformation|GetWorldRotation _cube)) (Variables|Default|GetForce)) "None" false))

(event EventTick
  (params (DeltaSeconds :type Float%20%28single-precision%29))
  (Variables|Default|SetLifeSpanCounter (+ (Variables|Default|GetLifeSpanCounter) DeltaSeconds))
  (if (>= (Variables|Default|GetLifeSpanCounter) (Variables|Default|GetLifeSpan))
    (Actor|DestroyActor)))

(fn ConstructionScript)

(fn JavlinHitting
  (params (Hit%20Object :type Actor%20Object%20Reference) (HitLocation :type Vector))
  (if (== (Utilities|GetClass Hit%20Object) "/Game/Characters/Dummy/BP_Dummy.BP_Dummy_C")
    (Development|PrintString "Dummy")
    (LocalVariables|SetPlayerPositionOnHit (Transformation|GetActorLocation (Game|Player|GetPlayerPawn 0)))
    (LocalVariables|SetEnemyPositionOnHit (Transformation|GetActorLocation Hit%20Object))
    (Transformation|SetActorLocation (Game|Player|GetPlayerPawn 0) (+ (/ (- (LocalVariables|GetEnemyPositionOnHit) (LocalVariables|GetPlayerPositionOnHit)) 2.2) (LocalVariables|GetPlayerPositionOnHit)) false false)
    (Transformation|SetActorLocation Hit%20Object (- (LocalVariables|GetEnemyPositionOnHit) (/ (- (LocalVariables|GetEnemyPositionOnHit) (LocalVariables|GetPlayerPositionOnHit)) 2.2)) false false)
    (Actor|DestroyActor)
    (else
      (Development|PrintString "Mur")
      (Transformation|SetActorLocation (Game|Player|GetPlayerPawn 0) HitLocation false false)
      (Actor|DestroyActor))))