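; BP_Javelin is a thrown spell projectile for Cramptix that teleports the player to wherever it hits.
; On BeginPlay it launches its physics Body with an impulse along its forward vector, scaled by Force.
; A hit on the Body moves player 0 to the javelin's location and destroys it, while Tick destroys it once LifeSpan elapses.
; An unfinished gradual-movement branch using vector slerp is never run.
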(event OnComponentHit(Body)
  (params (HitComponent :type Primitive%20Component%20Object%20Reference) (OtherActor :type Actor%20Object%20Reference) (OtherComp :type Primitive%20Component%20Object%20Reference) (NormalImpulse :type Vector :default "0, 0, 0") (Hit :type Hit%20Result%20Structure%20%28by%20ref%29))
  (Transformation|SetActorLocation (Game|Player|GetPlayerPawn 0) (Transformation|GetActorLocation) false false)
  (Actor|DestroyActor))

(event EventBeginPlay
  (bind _body (Variables|Default|GetBody))
  (Physics|AddImpulse _body (* (Math|Vector|GetForwardVector (Transformation|GetWorldRotation _body)) (Variables|Default|GetForce)) "None" false))

(event EventTick
  (params (DeltaSeconds :type Float%20%28single-precision%29))
  (Utilities|FlowControl|Sequence
    (:then_0
      (Variables|Default|SetLifeSpanCounter (+ (Variables|Default|GetLifeSpanCounter) DeltaSeconds))
      (if (>= (Variables|Default|GetLifeSpanCounter) (Variables|Default|GetLifeSpan))
        (Actor|DestroyActor)))
    (:then_1)))

(fn ConstructionScript)