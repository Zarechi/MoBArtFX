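; BP_Camptix_Clone is a clone of the Camptix character that travels straight ahead along its facing direction.
; Each Tick, while HasCollided is false, it reads SprintSpeed from the player's BP_Camptix and offsets its location by a scaled fraction of it.
; Movement is unswept and not scaled by delta time, so speed depends on frame rate.
; Nothing in these graphs sets HasCollided.
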(event EventTick
  (params (DeltaSeconds :type Float%20%28single-precision%29))
  (if (not (Variables|Default|GetHasCollided?))
    (bind _asbp_moba_character (Utilities|Casting|CastToBP_Camptix (Game|GetPlayerCharacter 0)))
    (Transformation|SetActorLocation (+ (Transformation|GetActorLocation) (* (Math|Vector|GetForwardVector (Transformation|GetActorRotation)) (/ (Variables|/Game/MOBA/BP/BP_Camptix.BP_Camptix_C|GetSprintSpeed _asbp_moba_character) 1e+02))) false false)))

(fn ConstructionScript)