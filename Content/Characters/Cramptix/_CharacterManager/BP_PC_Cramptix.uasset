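; BP_PC_Cramptix is the player controller for Cramptix that adds a double jump while the agility boost is on.
; On BeginPlay it caches the pawn as BP_Cramptix, printing an error if the cast fails.
; Pressing Jump while boosted and falling launches the character upward at its jump velocity and uses up the extra jump.
; The OnLandedCharacter event, which has no caller in this graph, restores it.
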(event Custom|OnLandedCharacter
  (Variables|Default|SetCanDoubleJump? true))

(event EventBeginPlay
  (bind _asbp_cramptix (Utilities|Casting|CastToBP_Cramptix (Game|Player|GetPlayerPawn 0))
    (:then
      (Variables|Default|SetBP_Cramptix _asbp_cramptix))
    (:CastFailed
      (Development|PrintString "BP_Cramptix cast failed !" true false "(R=1.000000,G=0.000000,B=0.099285,A=1.000000)" 3.0))))

(event EventTick
  (params (DeltaSeconds :type Float%20%28single-precision%29)))

(event Input|ActionEvents|InputActionJump
  (params (Key :type Key%20Structure :default "None"))
  (:Pressed
    (if (Math|Boolean|ANDBoolean (Variables|/Game/Characters/Cramptix/BP_Cramptix.BP_Cramptix_C|GetIsAgilityBoostOn? (Variables|Default|GetBP_Cramptix)) (AI|Components|NavMovement|IsFalling (Variables|/Script/Engine.Character|GetCharacterMovement (Variables|Default|GetBP_Cramptix))) (Variables|Default|GetCanDoubleJump?))
      (Character|LaunchCharacter (Variables|Default|GetBP_Cramptix) (Math|Vector|MakeVector 0.0 0.0 (Variables|/Script/Engine.CharacterMovementComponent|GetJumpZVelocity (Variables|/Script/Engine.Character|GetCharacterMovement (Variables|Default|GetBP_Cramptix)))) false false)
      (Variables|Default|SetCanDoubleJump? false))))

(fn ConstructionScript)