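; DesertClaw's Sunsetivities ability, which throws a grenade where the player aims.
; On run, it spawns BP_SunsetivitiesGrenade just along the camera trace, yawed to the control rotation, and launches its mesh with an impulse along the view, tilted slightly upward.
; An older shield-placement version remains disconnected: its stop and tick logic never runs, nor does the shield spawn that used GetPlacementLocationAndRotation's line traces to find valid ground.
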(event EventOnInitialize)

(event EventOnRun
  (params (context :type Moba%20Ability%20Run%20Context%20Structure))
  (bind _returnvalue (Class|MobaAbility|GetCharacter))
  (bind _returnvalue_2 (Class|DesertClawCharacter|GetPlayerController _returnvalue))
  (bind _returnvalue_3 (Pawn|GetControlRotation _returnvalue_2 :!class /Script/Engine.Controller))
  (bind (_start _end) (Class|PCMoBArtFX|GetCameraTraceBounds _returnvalue_2 15.0))
  (bind _returnvalue_4 (Game|SpawnActorfromClass "/Game/Characters/DesertClaw/Abilities/Sunsetivities/BP_SunsetivitiesGrenade.BP_SunsetivitiesGrenade_C" (Math|Transform|MakeTransform _end (Math|Rotator|MakeRotator 9e+01 0.0 (.yaw _returnvalue_3)) "1.000000,1.000000,1.000000") "Undefined" "MultiplyWithRoot" 0 (Math|Rotator|MakeRotator 0.0 0.0 (.yaw _returnvalue_3)) 0))
  (Physics|AddImpulse (Variables|/Game/Characters/DesertClaw/Abilities/Sunsetivities/BP_SunsetivitiesGrenade.BP_SunsetivitiesGrenade_C|GetMesh _returnvalue_4) (* (Math|Vector|Normalize (+ (- _end _start) "0.000000,0.000000,2.000000")) 5e+03) "None" false))

(event EventOnStop
  (params (context :type Moba%20Ability%20Run%20Context%20Structure))
  ;[0 0 0] old version
)

(event EventOnTick
  (params (delta_time :type Float%20%28single-precision%29))
  ;[0 0 0] old version
)

(fn GetPlacementLocationandRotation
  (bind _returnvalue (Class|MobaAbility|GetCharacter))
  (bind _shield_actor (Variables|Default|GetShield%20Actor))
  (bind _returnvalue_2 (Transformation|GetActorLocation _returnvalue))
  (bind _array (Utilities|Array|MakeArray _shield_actor))
  (Class|PCMoBArtFX|GetCameraTraceBounds (Class|DesertClawCharacter|GetPlayerController _returnvalue) 0.0)
  (bind (_outhit _returnvalue_3) (Collision|LineTraceByChannel "0, 0, 0" "0, 0, 0" "TraceTypeQuery1" false _array "ForOneFrame"))
  (if _returnvalue_3
    ;[1 1 1] Is Facing Up
    (if (Utilities|Operators|EqualEqual (.normal _outhit) "0.000000,0.000000,1.000000" 0.1)
      (return (.location _outhit) (Math|Rotator|MakeRotator 0.0 0.0 (.yaw (Math|Rotator|FindLookatRotation _returnvalue_2 (.location _outhit)))) true)
      (else
        (return (.location _outhit) (Math|Rotator|MakeRotator 0.0 0.0 (.yaw (Math|Rotator|FindLookatRotation _returnvalue_2 (.location _outhit)))) false)))
    (else
      (bind (_outhit_2 _returnvalue_4) (Collision|LineTraceByChannel "0, 0, 0" (+ "" (Math|Vector|MakeVector 0.0 0.0 (Variables|Default|GetPlacement%20Max%20Z%20Offset))) "TraceTypeQuery1" false _array "ForOneFrame"))
      (if _returnvalue_4
        (return (.location _outhit_2) (Math|Rotator|MakeRotator 0.0 0.0 (.yaw (Math|Rotator|FindLookatRotation _returnvalue_2 (.location _outhit_2)))) true)
        (else
          (return (.location _outhit_2) (Math|Rotator|MakeRotator 0.0 0.0 (.yaw (Math|Rotator|FindLookatRotation _returnvalue_2 (.location _outhit_2)))) false))))))