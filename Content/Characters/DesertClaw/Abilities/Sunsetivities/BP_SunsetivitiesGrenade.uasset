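; Grenade actor for DesertClaw's Sunsetivities ability, apparently meant to deploy a shield after landing, with that logic currently disconnected.
; The unwired nodes sketch a near-flat ground check that enables tick and damping, then a countdown that spawns and activates BP_SunsetivitiesShield.
; They would also bind the shield's end to destroying the grenade.
; As it stands, Tick is empty and only that destroy handler has a body.
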(event Custom|On%20Shield%20End%20Play
  (params (Actor :type Actor%20Object%20Reference) (EndPlayReason :type EEndPlayReason%20Enum :default "Destroyed"))
  ;[1 1 1] Spawn Shield
  (Actor|DestroyActor))

(event EventTick
  (params (DeltaSeconds :type Float%20%28single-precision%29)))

(fn ConstructionScript)