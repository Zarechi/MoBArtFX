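; Decal actor for DesertClaw's ultimate ability, providing pillar spawn locations and the fall sequence.
; Sequencer event endpoints forward next-pillar and end-fall cues to the ability, so sequence timing drives it.
; Getters expose the FallSequence component and the world location of one of seven spawn point components, selected by index.
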(event Custom|Trigger%20Next%20Pillar
  (params (Owner :type Actor%20Object%20Reference))
  (Class|DesertClawUltimateAbility|TriggerNextPillar (Class|DesertClawUltimateDecal|GetAbility)))

(event Custom|End%20Fall
  (params (Owner :type Actor%20Object%20Reference))
  (Class|DesertClawUltimateAbility|EndFall (Class|DesertClawUltimateDecal|GetAbility)))

(fn ConstructionScript)

(fn GetSpawnLocation
  (params (index :type Integer))
  (return (Transformation|GetWorldLocation (Utilities|Select :Index index :Option%200 (Variables|Default|GetSpawnPoint1) :Option%201 (Variables|Default|GetSpawnPoint2) :Option%202 (Variables|Default|GetSpawnPoint3) :Option%203 (Variables|Default|GetSpawnPoint4) :Option%204 (Variables|Default|GetSpawnPoint5) :Option%205 (Variables|Default|GetSpawnPoint6) :Option%206 (Variables|Default|GetSpawnPoint7)))))

(fn GetSequenceComponent
  (return (Variables|Default|GetFall%20Sequence)))