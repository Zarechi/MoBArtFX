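; DesertClaw's Cloud Nine ability, a two-press placement that spends sand from the passive to spawn a temporary sand cloud.
; In build mode, a pre-spawned hologram follows a camera trace, with a downward trace capping its height above ground, and shows cyan or red for affordability.
; An overridden-slot stop spawns the cloud at the hologram and destroys it after the cooldown delay.
; Any stop exits build mode and parks the hologram below the world.
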(event EventOnInitialize
  (CallFunction|SpawnandGetReferences))

(event EventOnRun
  (params (context :type Moba%20Ability%20Run%20Context%20Structure))
  (Variables|Default|SetisBuildModeActive true))

(event EventOnTick
  (params (delta_time :type Float%20%28single-precision%29))
  (if (Variables|Default|GetisBuildModeActive)
    (Utilities|FlowControl|Sequence
      (:then_0
        (bind (_ispositiongood _goodcloudposition) (CallFunction|TraceforCloud))
        (Development|PrintString (Utilities|String|ToString(Vector) _goodcloudposition))
        (if _ispositiongood
          (Transformation|SetActorLocation (Variables|CloudPlacement|GetHoloCloudReference) _goodcloudposition false false)))
      (:then_1
        (Rendering|Material|SetMaterial (Variables|/Game/Characters/DesertClaw/Abilities/CloudNine/BP_HologramCloud.BP_HologramCloud_C|GetCloudShape (Variables|CloudPlacement|GetHoloCloudReference)) 0 (select (Class|DesertClawPassiveAbility|CanAffordSand (Variables|Default|GetPassive) (Variables|Default|GetSandCost)) "/Game/Characters/DesertClaw/MaterialLibrary/MI_CyanTranslucent.MI_CyanTranslucent" "/Game/Characters/DesertClaw/MaterialLibrary/MI_RedTranslucent.MI_RedTranslucent"))))))

(event EventOnStop
  (params (context :type Moba%20Ability%20Run%20Context%20Structure))
  (if (.isoverridenslot context)
    (Utilities|FlowControl|Sequence
      (:then_0
        (if (Class|DesertClawPassiveAbility|CanAffordSand (Variables|Default|GetPassive) (Variables|Default|GetSandCost))
          (bind _returnvalue (Game|SpawnActorfromClass "/Game/Characters/DesertClaw/Abilities/CloudNine/BP_SandCloud.BP_SandCloud_C" (Math|Transform|MakeTransform (Transformation|GetActorLocation (Variables|CloudPlacement|GetHoloCloudReference)) "0, 0, 0" "1.000000,1.000000,1.000000") "AlwaysSpawn" "MultiplyWithRoot" 0 (Variables|SandCloud|GetSandCloudHeightCM) (Variables|SandCloud|GetSandCloudDiameterCM) 0))
          (Variables|SandCloud|SetSandCloudReference _returnvalue)
          (Class|DesertClawPassiveAbility|AddSandPercent (Variables|Default|GetPassive) (* (Variables|Default|GetSandCost) -1.0))
          (Utilities|FlowControl|Delay (Variables|/Script/MoBArtFX.MobaAbilityData|GetCooldown (Class|MobaAbility|GetData)))
          (Actor|DestroyActor (Variables|SandCloud|GetSandCloudReference))
          (else
            (Class|MobaAbility|SetCooldown 0.0))))
      (:then_1
        (Variables|Default|SetisBuildModeActive false :!label _label)
        (Transformation|SetActorLocation (Variables|CloudPlacement|GetHoloCloudReference) "0.000000,0.000000,-5000.000000" false false)))
    (else
      (Class|MobaAbility|SetCooldown 0.0)
      (goto _label))))

(fn SpawnandGetReferences
  (Utilities|FlowControl|Sequence
    (:then_0
      (bind _returnvalue (Game|SpawnActorfromClass "/Game/Characters/DesertClaw/Abilities/CloudNine/BP_HologramCloud.BP_HologramCloud_C" (Math|Transform|MakeTransform "0.000000,0.000000,-5000.000000" "0, 0, 0" "1.000000,1.000000,1.000000") "Undefined" "MultiplyWithRoot" 0 (Variables|SandCloud|GetSandCloudDiameterCM) (Variables|SandCloud|GetSandCloudHeightCM) 0))
      (Variables|CloudPlacement|SetHoloCloudReference _returnvalue))
    (:then_1
      (Variables|Default|SetActors%20to%20Ignore (Utilities|Array|MakeArray (Class|MobaAbility|GetCharacter)))
      (Variables|Default|SetPassive (.AsDesert%20Claw%20Passive%20Ability (Utilities|Casting|CastToDesertClawPassiveAbility (Class|DesertClawCharacter|GetAbility (Class|MobaAbility|GetCharacter) "Passive")))))))

(fn TraceforCloud
  (bind _array (Utilities|Array|MakeArray "ObjectTypeQuery1"))
  (bind (_start _end) (Class|PCMoBArtFX|GetCameraTraceBounds (Class|DesertClawCharacter|GetPlayerController (Class|MobaAbility|GetCharacter)) (Variables|Default|GetMaxHorizontalPlacementDistance)))
  (bind _output_get (LocalVariables|SetTraceStart _start))
  (bind _output_get_2 (LocalVariables|SetHypotheticalTraceEnd _end))
  (bind (_outhit _returnvalue) (Collision|LineTraceForObjects _output_get _output_get_2 _array false (Variables|Default|GetActors%20to%20Ignore) "ForOneFrame"))
  (if _returnvalue
    ;[0.4062 0.1189 0.3287] A Hit! Great! I guess...
    ; Rewind a little bit (to avoid being in the wall when you trace) and do the same as if you didn't hit!
    (LocalVariables|SetTraceHit (- (.ImpactPoint (Collision|BreakHitResult _outhit)) (Math|Vector|GetUnitDirection(Vector) (LocalVariables|GetTraceStart) (LocalVariables|GetHypotheticalTraceEnd))))
    (bind (_outhit_2 _returnvalue_2) (Collision|LineTraceForObjects (LocalVariables|GetTraceHit) (- (LocalVariables|GetTraceHit) (Math|Vector|MakeVector 0.0 0.0 5e+04)) _array false (Variables|Default|GetActors%20to%20Ignore) "None"))
    (if _returnvalue_2
      (if (<= (.Distance (Collision|BreakHitResult _outhit_2)) 3.5e+02)
        (return true (LocalVariables|GetTraceHit))
        (else
          ;[1 1 1] Other solution: just warp it downwards
          (return true (+ (.Location (Collision|BreakHitResult _outhit_2)) (Math|Vector|MakeVector 0.0 0.0 (Variables|Default|GetMaxPlacementHeight)))))))
    (else
      ;[0.4062 0.1189 0.3287] No hit, great!
      ; Now trace towards the ground to make sure you're not more than 350 away!
      (bind (_outhit_3 _returnvalue_3) (Collision|LineTraceForObjects (LocalVariables|GetHypotheticalTraceEnd) (- (LocalVariables|GetHypotheticalTraceEnd) (Math|Vector|MakeVector 0.0 0.0 5e+04)) _array false (Variables|Default|GetActors%20to%20Ignore) "None"))
      (if _returnvalue_3
        (if (<= (.Distance (Collision|BreakHitResult _outhit_3)) 3.5e+02)
          (return true (LocalVariables|GetHypotheticalTraceEnd))
          (else
            ;[1 1 1] Other solution: just warp it downwards
            (return true (+ (.Location (Collision|BreakHitResult _outhit_3)) (Math|Vector|MakeVector 0.0 0.0 (Variables|Default|GetMaxPlacementHeight))))))))))