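; BP_SandCloud is a sand cloud for DesertClaw's CloudNine ability that lifts an overlapping character up onto its top.
; On BeginPlay it scales itself from cylinder dimensions and passes a size-based value to the SandCloud effect.
; A DetectionPlatform overlap measures the feet-to-top distance and enables Tick, which zeroes velocity and teleports the character along a timed curve.
; It moves one character at a time and disables Tick when finished.
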(event OnComponentBeginOverlap(DetectionPlatform)
  (params (OverlappedComponent :type Primitive%20Component%20Object%20Reference) (OtherActor :type Actor%20Object%20Reference) (OtherComp :type Primitive%20Component%20Object%20Reference) (OtherBodyIndex :type Integer) (bFromSweep :type Boolean) (SweepResult :type Hit%20Result%20Structure%20%28by%20ref%29))
  (if (not (Variables|Default|GetbShouldMoveCharacterUp))
    (bind _ascharacter (Utilities|Casting|CastToCharacter OtherActor))
    (Variables|Default|SetTargetCharacter _ascharacter) ; In a real game this should probably be an Array and\nmove up all of them... but it's a prototype without multiplayer\nfor the moment so no
    (CallFunction|StartMovingCharacterUp)))

(event EventBeginPlay
  (CallFunction|ScaleActorfromParameters)
  (Actor|Tick|SetActorTickEnabled false))

(event EventTick
  (params (DeltaSeconds :type Float%20%28single-precision%29))
  (CallFunction|MoveOverlappedCharacter))

(fn ConstructionScript)

(fn ScaleActorfromParameters
  (bind _returnvalue (Transformation|GetActorScale3D))
  (bind _cylinderdiametercm (Variables|Default|GetCylinderDiameterCM))
  (bind _returnvalue_2 (/ _cylinderdiametercm 1e+02))
  (Transformation|SetActorScale3D (Math|Vector|MakeVector _returnvalue_2 _returnvalue_2 (/ (Variables|Default|GetCylinderHeightCM) 1e+02)))
  (Niagara|SetNiagaraVariable(Float) (Variables|Default|GetSandCloud) "ScaledNumber" (* (.x _returnvalue) (.z _returnvalue) 1e+03)))

(fn MoveOverlappedCharacter
  (bind _targetcharacterstartinglocation (Variables|Default|GetTargetCharacterStartingLocation))
  (CallFunction|IncreaseValueFloat (Variables|Default|GetcurrentMovementTimer) (Utilities|Time|GetWorldDeltaSeconds))
  ;[1 1 1] Stop all Forces
  (Variables|/Script/Engine.MovementComponent|SetVelocity (Variables|/Script/Engine.Character|GetCharacterMovement (Variables|Default|GetTargetCharacter)) "0, 0, 0")
  ;[1 1 1] Move Character
  (Transformation|SetActorLocation (Variables|Default|GetTargetCharacter) (Math|Vector|MakeVector (.x _targetcharacterstartinglocation) (.y _targetcharacterstartinglocation) (+ (.z _targetcharacterstartinglocation) (* (Math|Curves|GetFloatValue (Variables|Default|GetCurveToMoveCharacter) (/ (Variables|Default|GetcurrentMovementTimer) (Variables|Default|GetTimeToMoveCharacter))) (Variables|Default|GetDistanceToMoveCharacter)))) false true)
  (if (> (Variables|Default|GetcurrentMovementTimer) (Variables|Default|GetTimeToMoveCharacter))
    (CallFunction|FinishMovingCharacter)))

(fn FinishMovingCharacter
  (Variables|Default|SetbShouldMoveCharacterUp false)
  (Actor|Tick|SetActorTickEnabled false)
  (Variables|Default|SetcurrentMovementTimer 0.0))

(fn StartMovingCharacterUp
  (bind _targetcharacter (Variables|Default|GetTargetCharacter))
  (Variables|Default|SetbShouldMoveCharacterUp true)
  (Actor|Tick|SetActorTickEnabled true)
  ;[0.09375 0.04975 0.005811] Distance from character bottom to sand cloud top (but only take the Z axis):
  ; - Character bottom is CharacterLocation(Center) - CharacterScaledCapsuleHalfHeight
  ; - SandCloudTop is CloudLocation(Center) + CylinderRadiusCM
  ;
  ; Take only the height level of the two values (CharacterFeet & CloudTop). Since the character can only collide from the bottom of the cloud, it MUST be under it, so take CloudTop - CharacterFeet and it must be a positive value of the difference.
  (Variables|Default|SetDistanceToMoveCharacter (- (+ (.z (Transformation|GetActorLocation)) (/ (Variables|Default|GetCylinderHeightCM) 2.0)) (- (.z (Transformation|GetActorLocation _targetcharacter)) (Components|Capsule|GetScaledCapsuleHalfHeight (Variables|/Script/Engine.Character|GetCapsuleComponent _targetcharacter)))))
  (Variables|Default|SetcurrentMovementTimer 0.0)
  (Variables|Default|SetTargetCharacterStartingLocation (Transformation|GetActorLocation (Variables|Default|GetTargetCharacter))))