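; HUD for the Wukon Gustav character that passes player data to the viewport widget and displays cooldowns for two spells and the ultimate.
; Cooldown stores the duration and starts a looping timer for that slot at the current frame's delta time.
; Each tick reads the character's remaining cooldown to update the icon material's Alpha and the countdown text.
; At zero, it plays the slot's animation, hides the text and clears the timer.
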(event Custom|CustomEvent
  (bind _viewportinstance (Variables|Default|GetViewportInstance))
  (bind _character (Variables|Default|GetCharacter))
  (bind _returnvalue (Class|BaseCharacter|GetSpellCooldown _character "First"))
  (bind _aswbp_viewport_base (Utilities|Casting|CastToWBP_ViewportBase _viewportinstance))
  (bind _wbp_spellinfos (Variables|/Game/_GameManager/UI/WBP_ViewportBase.WBP_ViewportBase_C|GetWBP_SpellInfos _aswbp_viewport_base))
  (bind _txt_cd_01 (Variables|/Game/_GameManager/UI/WBP_SpellInfos.WBP_SpellInfos_C|GetTXT_CD_01 _wbp_spellinfos))
  (Rendering|Material|SetScalarParameterValue (Variables|/Game/_GameManager/UI/WBP_SpellInfos.WBP_SpellInfos_C|GetSpell01_DynMat _wbp_spellinfos) "Alpha" (- 1.0 (/ _returnvalue (Variables|Default|GetFirst%20Cooldown))) :!class /Script/Engine.MaterialInstanceDynamic)
  (Widget|SetVisibility _txt_cd_01 "Visible")
  (Rendering|Components|TextRender|SetText _txt_cd_01 (Utilities|Text|ToText(Float) _returnvalue "HalfToEven" false true 1 324 1 1))
  (if (<= _returnvalue 0.0)
    (UserInterface|Animation|PlayAnimation _wbp_spellinfos (Variables|/Game/_GameManager/UI/WBP_SpellInfos.WBP_SpellInfos_C|GetAnim_CD_01 _wbp_spellinfos) 0.0 1 "Forward" 1.0 false)
    (Widget|SetVisibility _txt_cd_01 "Hidden")
    (Utilities|Time|ClearandInvalidateTimerbyHandle (stale EventCooldown _returnvalue))))

(event Custom|CustomEvent_2
  (bind _viewportinstance (Variables|Default|GetViewportInstance))
  (bind _character (Variables|Default|GetCharacter))
  (bind _returnvalue (Class|BaseCharacter|GetSpellCooldown _character "Ultimate"))
  (bind _aswbp_viewport_base (Utilities|Casting|CastToWBP_ViewportBase _viewportinstance))
  (bind _wbp_spellinfos (Variables|/Game/_GameManager/UI/WBP_ViewportBase.WBP_ViewportBase_C|GetWBP_SpellInfos _aswbp_viewport_base))
  (bind _txt_cd_ult (Variables|/Game/_GameManager/UI/WBP_SpellInfos.WBP_SpellInfos_C|GetTXT_CD_Ult _wbp_spellinfos))
  (Rendering|Material|SetScalarParameterValue (Variables|/Game/_GameManager/UI/WBP_SpellInfos.WBP_SpellInfos_C|GetUltimate_DynMat _wbp_spellinfos) "Alpha" (- 1.0 (/ _returnvalue (Variables|Default|GetUltimate%20Cooldown))) :!class /Script/Engine.MaterialInstanceDynamic)
  (Widget|SetVisibility _txt_cd_ult "Visible")
  (Rendering|Components|TextRender|SetText _txt_cd_ult (Utilities|Text|ToText(Float) _returnvalue "HalfToEven" false true 1 324 1 1))
  (if (<= _returnvalue 0.0)
    (UserInterface|Animation|PlayAnimation _wbp_spellinfos (Variables|/Game/_GameManager/UI/WBP_SpellInfos.WBP_SpellInfos_C|GetAnim_CD_Ult _wbp_spellinfos) 0.0 1 "Forward" 1.0 false)
    (Widget|SetVisibility _txt_cd_ult "Hidden")
    (Utilities|Time|ClearandInvalidateTimerbyHandle (stale EventCooldown _returnvalue_3))))

(event Custom|CustomEvent_1
  (bind _viewportinstance (Variables|Default|GetViewportInstance))
  (bind _character (Variables|Default|GetCharacter))
  (bind _returnvalue (Class|BaseCharacter|GetSpellCooldown _character "Second"))
  (bind _aswbp_viewport_base (Utilities|Casting|CastToWBP_ViewportBase _viewportinstance))
  (bind _wbp_spellinfos (Variables|/Game/_GameManager/UI/WBP_ViewportBase.WBP_ViewportBase_C|GetWBP_SpellInfos _aswbp_viewport_base))
  (bind _txt_cd_02 (Variables|/Game/_GameManager/UI/WBP_SpellInfos.WBP_SpellInfos_C|GetTXT_CD_02 _wbp_spellinfos))
  (Rendering|Material|SetScalarParameterValue (Variables|/Game/_GameManager/UI/WBP_SpellInfos.WBP_SpellInfos_C|GetSpell02_DynMat _wbp_spellinfos) "Alpha" (- 1.0 (/ _returnvalue (Variables|Default|GetSecond%20Cooldown))) :!class /Script/Engine.MaterialInstanceDynamic)
  (Widget|SetVisibility _txt_cd_02 "Visible")
  (Rendering|Components|TextRender|SetText _txt_cd_02 (Utilities|Text|ToText(Float) _returnvalue "HalfToEven" false true 1 324 1 1))
  (if (<= _returnvalue 0.0)
    (UserInterface|Animation|PlayAnimation _wbp_spellinfos (Variables|/Game/_GameManager/UI/WBP_SpellInfos.WBP_SpellInfos_C|GetAnim_CD_02 _wbp_spellinfos) 0.0 1 "Forward" 1.0 false)
    (Widget|SetVisibility _txt_cd_02 "Hidden")
    (Utilities|Time|ClearandInvalidateTimerbyHandle (stale EventCooldown _returnvalue_2))))

(event EventCooldown
  (params (time :type Float%20%28single-precision%29) (type :type EMobaAbilitySlot%20Enum :default "First"))
  (switch Utilities|FlowControl|Switch|SwitchonEMobaAbilitySlot type
    (:First
      (Variables|Default|SetFirst%20Cooldown time)
      (bind _returnvalue (Utilities|Time|SetTimerbyEvent (delegate Custom|CustomEvent) (Utilities|Time|GetWorldDeltaSeconds) true)))
    (:Second
      (Variables|Default|SetSecond%20Cooldown time)
      (bind _returnvalue_2 (Utilities|Time|SetTimerbyEvent (delegate Custom|CustomEvent_1) (Utilities|Time|GetWorldDeltaSeconds) true)))
    (:Ultimate
      (Variables|Default|SetUltimate%20Cooldown time)
      (bind _returnvalue_3 (Utilities|Time|SetTimerbyEvent (delegate Custom|CustomEvent_2) (Utilities|Time|GetWorldDeltaSeconds) true)))))

(event EventBeginPlay
  (Variables|Default|SetCharacter (.AsBase%20Character (Utilities|Casting|CastToBaseCharacter (Pawn|GetControlledPawn (Game|Player|GetOwningPlayerController))))))

(event EventSetViewportPlayerDatas
  (bind _asbase_character (Utilities|Casting|CastToBaseCharacter (Pawn|GetControlledPawn (Game|Player|GetOwningPlayerController))))
  (Default|SetPlayerDatas (.AsWBP%20Viewport%20Base (Utilities|Casting|CastToWBP_ViewportBase (Variables|Default|GetViewportInstance))) (Class|BaseCharacter|GetPlayerDatas _asbase_character)))

(fn ConstructionScript)