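; BP_Smoke is a temporary smoke area for the Gustav character that damages actors inside it and destroys itself after ten seconds.
; Box overlap events add and remove actors in a tracked array.
; Tick runs through a Delay, acting as a half-second pulse that calls ApplyMobaDamage on each tracked actor except the owner.
; The owner, cast to BaseCharacter, is credited as instigator; an unconnected ApplyDamage call remains unused.
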(event OnComponentBeginOverlap(Box)
  (params (OverlappedComponent :type Primitive%20Component%20Object%20Reference) (OtherActor :type Actor%20Object%20Reference) (OtherComp :type Primitive%20Component%20Object%20Reference) (OtherBodyIndex :type Integer) (bFromSweep :type Boolean) (SweepResult :type Hit%20Result%20Structure%20%28by%20ref%29))
  (Utilities|Array|AddUnique (Variables|Default|GetOther%20Actor) OtherActor))

(event OnComponentEndOverlap(Box)
  (params (OverlappedComponent :type Primitive%20Component%20Object%20Reference) (OtherActor :type Actor%20Object%20Reference) (OtherComp :type Primitive%20Component%20Object%20Reference) (OtherBodyIndex :type Integer))
  (Utilities|Array|RemoveItem (Variables|Default|GetOther%20Actor) OtherActor))

(event EventTick
  (params (DeltaSeconds :type Float%20%28single-precision%29))
  (bind _returnvalue (Components|GetOwner))
  (Utilities|FlowControl|Delay 0.5)
  (for _array_element (Variables|Default|GetOther%20Actor)
    (if (not (== _array_element _returnvalue))
      (bind _asbase_character (Utilities|Casting|CastToBaseCharacter _returnvalue))
      (Class|MobaGameplayStatics|ApplyMobaDamage _array_element 15.0 self _asbase_character))))

(event EventBeginPlay
  (Utilities|FlowControl|Delay 1e+01)
  (Utilities|Array|Clear (Variables|Default|GetOther%20Actor))
  (Actor|DestroyActor))

(fn ConstructionScript)