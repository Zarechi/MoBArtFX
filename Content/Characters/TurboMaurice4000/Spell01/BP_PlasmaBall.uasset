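; BP_PlasmaBall is TurboMaurice4000's plasma ball spell, extending its parent's damage logic with a combo against BP_Rocket.
; Ordinary hits apply direct damage, while hitting a rocket destroys it and triggers a plasma explosion with radial falloff damage scaled from the capsule size.
; A sphere trace then gives each new pawn except the instigator a damage-over-time component and knocks characters outward and upward.
; An optional debug flag draws both blast radii.
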(fn ConstructionScript)

(fn DoDamages
  (params (HitActor :type Actor%20Object%20Reference) (HitComponent :type Actor%20Component%20Object%20Reference))
  (bind _capsule (Variables|Default|GetCapsule))
  (bind _capsule_2 (Variables|Default|GetCapsule))
  (bind _damages (Variables|Default|GetDamages))
  (bind _hitlocation (Variables|Default|GetHitLocation))
  (bind _returnvalue (Components|Capsule|GetScaledCapsuleHalfHeight _capsule_2))
  (bind _returnvalue_2 (Components|Capsule|GetScaledCapsuleHalfHeight _capsule))
  (|CallParentFunction HitActor HitComponent)
  (bind _asbp_rocket (Utilities|Casting|CastToBP_Rocket HitActor)
    (:then
      (Utilities|IsValid _asbp_rocket
        (:Is%20Valid
          (Actor|DestroyActor HitActor)
          (Niagara|SpawnSystematLocation "/Game/Characters/TurboMaurice4000/Spell01/FX/NS_PlasmaExplosion.NS_PlasmaExplosion" (Variables|Default|GetHitLocation))
          (Class|GameplayStatics|ApplyRadialDamagewithFalloff _damages (/ _damages 1e+01) (Variables|Default|GetHitLocation) _returnvalue (* _returnvalue (Variables|Default|GetAreaFactor)) 5.0 "/Game/Characters/TurboMaurice4000/Spell01/DT_PlasmaExplosion.DT_PlasmaExplosion_C" (Utilities|Array|MakeArray self) (Variables|Default|GetInstigator) (Game|GetInstigatorController) "ECC_Visibility")
          (bind _outhits (Collision|MultiSphereTraceForObjects _hitlocation _hitlocation (* (Components|Capsule|GetScaledCapsuleHalfHeight (Variables|Default|GetCapsule)) (Variables|Default|GetAreaFactor)) (Utilities|Array|MakeArray "ObjectTypeQuery3") false (Utilities|Array|MakeArray self) "None"))
          (Utilities|Array|AddUnique (LocalVariables|GetHitActors) (Variables|Default|GetInstigator))
          (for _array_element _outhits
            (if (not (Utilities|Array|ContainsItem (LocalVariables|GetHitActors) (.HitActor (Collision|BreakHitResult _array_element))))
              (Utilities|Array|AddUnique (LocalVariables|GetHitActors) (.HitActor (Collision|BreakHitResult _array_element)))
              (Game|AddComponentbyClass (.HitActor (Collision|BreakHitResult _array_element)) "/Game/_GameManager/ActorComponents/AC_DoT.AC_DoT_C" 0.5)
              (bind _ascharacter (Utilities|Casting|CastToCharacter (.HitActor (Collision|BreakHitResult _array_element))))
              (Physics|AddImpulse (Variables|/Script/Engine.Character|GetCharacterMovement _ascharacter) (* (Math|Vector|Normalize (+ (- (Transformation|GetActorLocation (.HitActor (Collision|BreakHitResult _array_element))) (Transformation|GetActorLocation)) "0.000000,0.000000,500.000000")) 5e+02) true)))
          (if (Variables|Default|GetDebugAreas)
            (Rendering|Debug|DrawDebugSphere (Variables|Default|GetHitLocation) _returnvalue_2 12 "(R=1.000000,G=0.000000,B=0.000000,A=1.000000)" 5.0 5.0)
            (Rendering|Debug|DrawDebugSphere (Variables|Default|GetHitLocation) (* _returnvalue_2 (Variables|Default|GetAreaFactor)) 12 "(R=0.109375,G=0.000000,B=0.000000,A=1.000000)" 5.0 5.0)))))
    (:CastFailed
      (Game|Damage|ApplyDamage HitActor (Variables|Default|GetDamages) (Game|GetInstigatorController) (Variables|Default|GetInstigator)))))