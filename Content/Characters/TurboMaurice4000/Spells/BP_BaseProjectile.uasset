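; Base projectile for TurboMaurice4000 spells that detects hits along its path and destroys itself on impact.
; Each tick it sphere-traces from its previous location to the current one, sized by the capsule half-height and ignoring the instigator, so movement between frames is covered.
; A blocking hit stores the hit location and calls DoDamages, which is empty here, before the projectile is destroyed.
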(event EventBeginPlay
  (Variables|Default|SetPreviousLocation (Transformation|GetActorLocation)))

(event EventTick
  (params (DeltaSeconds :type Float%20%28single-precision%29))
  (bind _outhit (Collision|SphereTraceForObjects (Variables|Default|GetPreviousLocation) (Transformation|GetActorLocation) (Components|Capsule|GetScaledCapsuleHalfHeight (Variables|Default|GetCapsule)) (Utilities|Array|MakeArray "ObjectTypeQuery1" "ObjectTypeQuery2" "ObjectTypeQuery3") false (Utilities|Array|MakeArray (Variables|Actor|GetInstigator)) "None"))
  (Variables|Default|SetPreviousLocation (Transformation|GetActorLocation))
  (if (.bBlockingHit (Collision|BreakHitResult _outhit))
    (Variables|Default|SetHitLocation (.Location (Collision|BreakHitResult _outhit)))
    (CallFunction|DoDamages (.HitActor (Collision|BreakHitResult _outhit)) (.HitComponent (Collision|BreakHitResult _outhit)))
    (Actor|DestroyActor) ; Then destroy this projectile
  ))

(fn ConstructionScript)

(fn DoDamages
  (params (HitActor :type Actor%20Object%20Reference) (HitComponent :type Actor%20Component%20Object%20Reference)))