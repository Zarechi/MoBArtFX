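; TurboMaurice4000 playable character, with camera-aimed rocket auto-attack, plasma ball, grab dash and charged ultimate.
; Abilities pass permission checks and start cooldowns; projectiles aim through a camera sphere trace.
; Timers drive the dash, which attaches hit characters until it ends, and the ultimate, which holds a holoshield before firing.
; Damage taken during the ultimate accumulates partly in AbsorbedDamages, though any damage currently zeroes health.
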(event Custom|HitEvent
  (params (SelfActor :type Actor%20Object%20Reference) (OtherActor :type Actor%20Object%20Reference) (NormalImpulse :type Vector) (Hit :type Hit%20Result%20Structure%20%28by%20ref%29))
  (bind _asbase_character (Utilities|Casting|CastToBaseCharacter OtherActor))
  (Utilities|Array|AddUnique (Variables|Default|GetGrabbedCharacters) _asbase_character)
  (Transformation|AttachActorToActor _asbase_character self "" "KeepWorld" "KeepWorld" "KeepRelative" true)
  (Collision|SetCollisionResponsetoAllChannels (Variables|/Script/Engine.Character|GetCapsuleComponent _asbase_character) "ECR_Overlap")
  (Variables|/Script/Engine.CharacterMovementComponent|SetGravityScale (Variables|/Script/Engine.Character|GetCharacterMovement _asbase_character) 0.0)
  (Niagara|SpawnSystematLocation "/Game/Characters/TurboMaurice4000/Spells/Spell02/FX/Grab/NS_ky_flash1.NS_ky_flash1" (Transformation|GetActorLocation _asbase_character)))

(event Custom|Dash
  (Character|LaunchCharacter (+ (* (Transformation|GetActorForwardVector) (Variables|Default|GetDashSpeed)) "0.000000,0.000000,1.000000") false true)
  (if (>= (- (Utilities|Time|GetRealTimeSeconds) (Variables|Default|GetCastTimeS2)) (Variables|Default|GetDashTimeS2))
    (Utilities|Time|ClearandInvalidateTimerbyHandle (stale EventSpell02 _returnvalue_2))
    (EventDispatchers|UnbindallEventsfromOnActorHit)
    (Components|DestroyComponent (stale EventSpell02 _returnvalue_3))
    (for _array_element (Variables|Default|GetGrabbedCharacters)
      (Transformation|DetachFromActor _array_element "KeepWorld" "KeepWorld" "KeepRelative")
      (Collision|SetCollisionResponsetoAllChannels (Variables|/Script/Engine.Character|GetCapsuleComponent _array_element) "ECR_Block")
      (Variables|/Script/Engine.CharacterMovementComponent|SetGravityScale (Variables|/Script/Engine.Character|GetCharacterMovement _array_element) 1.0))))

(event Custom|Cast
  (bind _returnvalue (Utilities|Time|GetRealTimeSeconds))
  (bind _casttimeultimate (Variables|Default|GetCastTimeUltimate))
  (bind _castdurationultimate (Variables|Default|GetCastDurationUltimate))
  (bind _returnvalue_2 (- _returnvalue _casttimeultimate))
  (bind _returnvalue_3 (>= _returnvalue_2 _castdurationultimate))
  (Variables|Default|SetUltiON? (not _returnvalue_3))
  (if _returnvalue_3
    (Utilities|Time|ClearandInvalidateTimerbyHandle (stale EventUltimate _returnvalue_2))
    (Components|DestroyComponent (Variables|/Game/Characters/TurboMaurice4000/Spells/Ultimate/FX/Blueprint/AC_Holoshield.AC_Holoshield_C|GetSkeletalMeshComp (stale EventUltimate _returnvalue_3)))
    (Components|DestroyComponent (stale EventUltimate _returnvalue_3))
    (bind _outhit (CallFunction|ForwardTrace 3e+01))
    (Game|SpawnActorfromClass (Variables|Default|GetUltimateProjectile) (Math|Transform|MakeTransform (.location (Transformation|GetSocketTransform (Variables|Character|GetMesh) (Variables|Default|Getultimate_socket) "RTS_World")) (Math|Rotator|FindLookatRotation (.TraceStart (Collision|BreakHitResult _outhit)) (Math|Vector|SelectVector (.Location (Collision|BreakHitResult _outhit)) (.TraceEnd (Collision|BreakHitResult _outhit)) (.bBlockingHit (Collision|BreakHitResult _outhit)))) "1.000000,1.000000,1.000000") "Undefined" "MultiplyWithRoot" 0 self)
    (Variables|/Script/Engine.CharacterMovementComponent|SetMaxWalkSpeed (Variables|Character|GetCharacterMovement) (Variables|Default|GetMax%20Walk%20Speed))))

(event EventAutoAttack
  (bind _returnvalue (Game|GetPlayerController 0))
  (bind _mesh (Variables|Character|GetMesh))
  (bind _left_fire_socket (Variables|Default|Getleft_fire_socket))
  (bind _returnvalue_2 (Transformation|GetSocketTransform _mesh _left_fire_socket "RTS_World"))
  (bind _asbp_pc_mo_bart_fx (Utilities|Casting|CastToBP_PC_MoBArtFX _returnvalue))
  (|CallParentFunction)
  (Utilities|HasPermission? (Variables|/Game/_GameManager/BP_PC_MoBArtFX.BP_PC_MoBArtFX_C|GetGameplay%20State _asbp_pc_mo_bart_fx) (Variables|/Script/MoBArtFX.PC_MoBArtFX|GetAutoAttackAction _asbp_pc_mo_bart_fx)
    (:HasPermission
      (if (> (Variables|/Script/MoBArtFX.PlayerInfos|GetCurrentAmmo (Class|BaseCharacter|GetPlayerDatas)) 0)
        (Utilities|Cooldown (Variables|/Script/MoBArtFX.PlayerInfos|GetAutoAttack_CD (Class|BaseCharacter|GetPlayerDatas)) -1)
        (bind _outhit (CallFunction|ForwardTrace 3e+01))
        (Game|SpawnActorfromClass "/Game/Characters/TurboMaurice4000/Spells/Auto-Attack/BP_Rocket.BP_Rocket_C" (Math|Transform|MakeTransform (.location _returnvalue_2) (Math|Rotator|SelectRotator (Math|Rotator|FindLookatRotation (.location _returnvalue_2) (.Location (Collision|BreakHitResult _outhit))) (Camera|GetCameraRotation (Game|GetPlayerCameraManager 0)) (.bBlockingHit (Collision|BreakHitResult _outhit))) "1.000000,1.000000,1.000000") "Undefined" "MultiplyWithRoot" 0 7e+02 self)))))

(event EventBeginPlay
  (|CallParentFunction)
  (Components|SkinnedMesh|HideBonebyName (Variables|Character|GetMesh) "head" "PBO_None"))

(event EventUltimate
  (bind _returnvalue (Game|GetPlayerController 0))
  (bind _asbp_pc_mo_bart_fx (Utilities|Casting|CastToBP_PC_MoBArtFX _returnvalue))
  (|CallParentFunction)
  (Utilities|HasPermission? (Variables|/Game/_GameManager/BP_PC_MoBArtFX.BP_PC_MoBArtFX_C|GetGameplay%20State _asbp_pc_mo_bart_fx) (Variables|/Script/MoBArtFX.PC_MoBArtFX|GetUltimateAction _asbp_pc_mo_bart_fx)
    (:HasPermission
      (Utilities|Cooldown (Variables|/Script/MoBArtFX.PlayerInfos|GetUltimate_CD (Class|BaseCharacter|GetPlayerDatas)) 2)
      (Variables|Default|SetAbsorbedDamages 0.0)
      (Variables|/Script/Engine.CharacterMovementComponent|SetMaxWalkSpeed (Variables|Character|GetCharacterMovement) (Variables|Default|GetMax%20Walk%20Speed_Ultimate))
      (bind _returnvalue_2 (Utilities|Time|SetTimerbyEvent (delegate Custom|Cast) (Utilities|Time|GetWorldDeltaSeconds) true))
      (Variables|Default|SetCastTimeUltimate (Utilities|Time|GetRealTimeSeconds))
      (bind _returnvalue_3 (Game|AddComponentbyClass "/Game/Characters/TurboMaurice4000/Spells/Ultimate/FX/Blueprint/AC_Holoshield.AC_Holoshield_C")))))

(event Game|Damage|EventAnyDamage
  (params (Damage :type Float%20%28single-precision%29) (DamageType :type Damage%20Type%20Object%20Reference) (InstigatedBy :type Controller%20Object%20Reference) (DamageCauser :type Actor%20Object%20Reference))
  (Variables|/Script/MoBArtFX.PlayerInfos|SetCurrentHealth (Class|BaseCharacter|GetPlayerDatas) 0.0 (Math|Integer|Max(Integer) (Math|Float|Truncate (- (.CurrentHealth (Variables|/Script/MoBArtFX.PlayerInfos|GetCurrentHealth (Class|BaseCharacter|GetPlayerDatas))) (Math|Float|SelectFloat (* Damage 0.75) Damage (Variables|Default|GetUltiON?))))))
  (if (Variables|Default|GetUltiON?)
    (Variables|Default|SetAbsorbedDamages (+ (* Damage 0.25) (Variables|Default|GetAbsorbedDamages)))))

(event EventSpell01
  (bind _returnvalue (Game|GetPlayerController 0))
  (bind _asbp_pc_mo_bart_fx (Utilities|Casting|CastToBP_PC_MoBArtFX _returnvalue))
  (|CallParentFunction)
  (Utilities|HasPermission? (Variables|/Game/_GameManager/BP_PC_MoBArtFX.BP_PC_MoBArtFX_C|GetGameplay%20State _asbp_pc_mo_bart_fx) (Variables|/Script/MoBArtFX.PC_MoBArtFX|GetSpell01_Action _asbp_pc_mo_bart_fx)
    (:HasPermission
      (Utilities|Cooldown (Variables|/Script/MoBArtFX.PlayerInfos|GetSpell01_CD (Class|BaseCharacter|GetPlayerDatas)) 0)
      (bind _outhit (CallFunction|ForwardTrace 3e+01))
      (Game|SpawnActorfromClass "/Game/Characters/TurboMaurice4000/Spells/Spell01/BP_PlasmaBall.BP_PlasmaBall_C" (Math|Transform|MakeTransform (.location (Transformation|GetSocketTransform (Variables|Character|GetMesh) (Variables|Default|Getright_fire_socket) "RTS_World")) (Math|Rotator|FindLookatRotation (.TraceStart (Collision|BreakHitResult _outhit)) (Math|Vector|SelectVector (.Location (Collision|BreakHitResult _outhit)) (.TraceEnd (Collision|BreakHitResult _outhit)) (.bBlockingHit (Collision|BreakHitResult _outhit)))) "1.000000,1.000000,1.000000") "Undefined" "MultiplyWithRoot" 0 1e+02 self))))

(event EventSpell02
  (bind _returnvalue (Game|GetPlayerController 0))
  (bind _asbp_pc_mo_bart_fx (Utilities|Casting|CastToBP_PC_MoBArtFX _returnvalue))
  (|CallParentFunction)
  (Utilities|HasPermission? (Variables|/Game/_GameManager/BP_PC_MoBArtFX.BP_PC_MoBArtFX_C|GetGameplay%20State _asbp_pc_mo_bart_fx) (Variables|/Script/MoBArtFX.PC_MoBArtFX|GetSpell01_Action _asbp_pc_mo_bart_fx)
    (:HasPermission
      (Utilities|Cooldown (Variables|/Script/MoBArtFX.PlayerInfos|GetSpell02_CD (Class|BaseCharacter|GetPlayerDatas)) 1)
      (bind _returnvalue_2 (Utilities|Time|SetTimerbyEvent (delegate Custom|Dash) (Utilities|Time|GetWorldDeltaSeconds) true))
      (Variables|Default|SetCastTimeS2 (Utilities|Time|GetRealTimeSeconds))
      (Collision|BindEventtoOnActorHit (delegate Custom|HitEvent))
      (bind _returnvalue_3 (Niagara|SpawnSystemAttached "/Game/Characters/TurboMaurice4000/Spells/Spell02/FX/Dash/NS_Energy.NS_Energy" (Variables|Character|GetMesh) "None" "0, 0, 0" "0, 0, 0" "KeepRelativeOffset" false)))))

(event Input|KeyboardEvents|DebugKeyH
  (params (Key :type Key%20Structure :default "None") (ActionValue :type Input%20Action%20Value%20Structure))
  (bind _returnvalue (Class|BaseCharacter|GetPlayerDatas))
  (:Pressed
    (Variables|/Script/MoBArtFX.PlayerInfos|SetCurrentHealth _returnvalue 0.0 (- (.CurrentHealth (Variables|/Script/MoBArtFX.PlayerInfos|GetCurrentHealth _returnvalue)) (Math|Random|RandomInteger 10)))))

(fn ConstructionScript
  (|CallParentFunction))

(fn ForwardTrace
  (params (Radius :type Float%20%28single-precision%29))
  (bind _returnvalue (Game|GetPlayerCameraManager 0))
  (bind _returnvalue_2 (Camera|GetCameraLocation _returnvalue))
  (bind _outhit (Collision|SphereTraceForObjects _returnvalue_2 (+ _returnvalue_2 (* (Math|Vector|GetForwardVector (Camera|GetCameraRotation _returnvalue)) 1e+04)) Radius (Variables|Default|GetAffectedChannels) false 0 "None"))
  (return _outhit))