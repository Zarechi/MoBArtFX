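; BP_Rocket is the rocket for TurboMaurice4000's auto-attack, dealing area damage on impact.
; It overrides DoDamages, calling the parent, then spawning an impact particle and applying radial damage with falloff at the hit location.
; The capsule half-height sets the inner radius, AreaFactor scales it for the outer radius, and DebugAreas draws both as debug spheres.
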(fn ConstructionScript
  (|CallParentFunction))

(fn DoDamages
  (params (HitActor :type Actor%20Object%20Reference) (HitComponent :type Actor%20Component%20Object%20Reference))
  (bind _capsule (Variables|Default|GetCapsule))
  (bind _damages (Variables|Default|GetDamages))
  (bind _capsule_2 (Variables|Default|GetCapsule))
  (bind _returnvalue (Components|Capsule|GetScaledCapsuleHalfHeight _capsule))
  (bind _returnvalue_2 (Components|Capsule|GetScaledCapsuleHalfHeight _capsule_2))
  (|CallParentFunction HitActor HitComponent)
  (Effects|SpawnEmitteratLocation "/Game/Characters/TurboMaurice4000/FX/Particles/Abilities/Cross/FX/P_Crunch_Cross_Impact.P_Crunch_Cross_Impact" (Variables|Default|GetHitLocation) "0, 0, 0" "1.500000,1.500000,1.500000")
  (Class|GameplayStatics|ApplyRadialDamagewithFalloff _damages (/ _damages 1e+01) (Variables|Default|GetHitLocation) _returnvalue_2 (* _returnvalue_2 (Variables|Default|GetAreaFactor)) 5.0 "/Script/Engine.DamageType" (Utilities|Array|MakeArray self) (Variables|Default|GetInstigator) (Game|GetInstigatorController) "ECC_Visibility")
  (if (Variables|Default|GetDebugAreas)
    (Rendering|Debug|DrawDebugSphere (Variables|Default|GetHitLocation) _returnvalue 12 "(R=1.000000,G=0.000000,B=0.000000,A=1.000000)" 5.0 5.0)
    (Rendering|Debug|DrawDebugSphere (Variables|Default|GetHitLocation) (* _returnvalue (Variables|Default|GetAreaFactor)) 12 "(R=0.109375,G=0.000000,B=0.000000,A=1.000000)" 5.0 5.0)))