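; Actor component that gives its owner a holoshield effect by overlaying a duplicate mesh, part of TurboMaurice4000's ultimate FX.
; On BeginPlay it finds the owner's MeshComponent and adds a component of the same class and relative transform.
; Skeletal copies take the source asset and anim class, with the holoshield material on every slot.
; Static copies take the mesh and world transform, with the material on slot 0 only.
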(event EventBeginPlay
  (bind _output_get (Variables|Default|SetMeshToShield (Actor|GetComponentbyClass (Components|GetOwner) "/Script/Engine.MeshComponent")))
  (bind _returnvalue (Game|AddComponentbyClass (Components|GetOwner) (Utilities|GetClass _output_get) false (Transformation|GetRelativeTransform _output_get)))
  (Utilities|DetectMesh _returnvalue
    (:IsSkeletal
      (CallFunction|SetSkeletalsShield))
    (:IsStatic
      (CallFunction|SetStaticShield))
    (:Undefined
      (Development|PrintString (Utilities|String|Append "Can't find a MeshComponent in " (Utilities|GetDisplayName (Components|GetOwner)))))))

(fn SetSkeletalsShield
  (bind _skeletalmeshcomp (Variables|Default|GetSkeletalMeshComp))
  (bind _output_get (LocalVariables|SetSkeletalMeshToShield (.AsSkeletal%20Mesh%20Component (Utilities|Casting|CastToSkeletalMeshComponent (Variables|Default|GetMeshToShield)))))
  (Components|SkinnedMesh|SetSkinnedAssetandUpdate (Variables|Default|GetSkeletalMeshComp) (Components|SkeletalMesh|GetSkeletalMeshAsset _output_get) true)
  (Class|SkeletalMeshComponent|SetAnimClass (Variables|Default|GetSkeletalMeshComp) (Variables|/Script/Engine.SkeletalMeshComponent|GetAnimClass (LocalVariables|GetSkeletalMeshToShield)))
  (for _index (range 0 (Rendering|Material|GetNumMaterials _skeletalmeshcomp))
    (Rendering|Material|SetMaterial _skeletalmeshcomp _index "/Game/Characters/TurboMaurice4000/Ultimate/FX/Materials/MI_Holoshield_New.MI_Holoshield_New")))

(fn SetStaticShield
  (bind _asstatic_mesh_component (Utilities|Casting|CastToStaticMeshComponent (Variables|Default|GetMeshToShield)))
  (bind _output_get (LocalVariables|SetStaticMeshToShield _asstatic_mesh_component))
  (Components|StaticMesh|SetStaticMesh (Variables|Default|GetStaticMeshComp) (Variables|/Script/Engine.StaticMeshComponent|GetStaticMesh _output_get))
  (Rendering|Material|SetMaterial (Variables|Default|GetStaticMeshComp) 0 "/Game/Characters/TurboMaurice4000/Ultimate/FX/Materials/MI_Holoshield_New.MI_Holoshield_New")
  (Transformation|SetWorldTransform (Variables|Default|GetStaticMeshComp) (Transformation|GetWorldTransform (LocalVariables|GetStaticMeshToShield)) false false))