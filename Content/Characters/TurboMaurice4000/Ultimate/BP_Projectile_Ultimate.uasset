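; Ultimate projectile for the TurboMaurice4000 character, whose damage grows with the amount of damage absorbed.
; It overrides DoDamages, running the parent logic, then applying damage to the hit actor with the instigator as causer.
; Total damage is a minimum plus a bonus scaled by absorbed damage, clamped at a maximum absorbed amount.
; The event graph holds only disabled placeholder events.
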(event EventBeginPlay
  (|CallParentFunction) ; This node is disabled and will not be called.\nDrag off pins to build functionality.
)

(event Collision|EventActorBeginOverlap
  (params (OtherActor :type Actor%20Object%20Reference)))

(event EventTick
  (params (DeltaSeconds :type Float%20%28single-precision%29))
  (|CallParentFunction DeltaSeconds) ; This node is disabled and will not be called.\nDrag off pins to build functionality.
)

(fn ConstructionScript
  (|CallParentFunction))

(fn DoDamages
  (params (HitActor :type Actor%20Object%20Reference) (HitComponent :type Actor%20Component%20Object%20Reference))
  (|CallParentFunction HitActor HitComponent)
  (bind _output_get (LocalVariables|SetTotalDamages (+ (Variables|Default|GetMinDamages) (* (Variables|Default|GetDamages) (Math|Float|MapRangeClamped (Variables|Default|GetAbsorbedDamages) 0.0 (Variables|Default|GetMaxAbsorbedDamages) 0.0 1.0)))))
  (Game|Damage|ApplyDamage HitActor _output_get (Game|GetInstigatorController) (Variables|Default|GetInstigator)))