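; BP_Needle is a needle that acts on sphere overlap as a normal hit, skill shot or teleport, tracking the Player it belongs to.
; Against other BaseCharacters it calls Hit or SkillShotHit (slow and stun delays) on their Needle_Damage_System component, then destroys itself.
; Overlapping a non-character destroys it, first moving the Player to its location if it is a teleport needle.
; An unconnected copy of this logic targeting BP_NeedlePlayer directly remains in the graph.
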(event OnComponentBeginOverlap(Sphere1)
  (params (OverlappedComponent :type Primitive%20Component%20Object%20Reference) (OtherActor :type Actor%20Object%20Reference) (OtherComp :type Primitive%20Component%20Object%20Reference) (OtherBodyIndex :type Integer) (bFromSweep :type Boolean) (SweepResult :type Hit%20Result%20Structure%20%28by%20ref%29))
  (bind _player (Variables|Default|GetPlayer))
  (bind _asbase_character (Utilities|Casting|CastToBaseCharacter OtherActor)
    (:then
      (Variables|Default|SetDamageSystem (Actor|GetComponentbyClass _asbase_character "/Script/MoBArtFX.Needle_Damage_System"))
      ;[1 1 1] Check if player is valid
      (if (!= OtherActor _player)
        (if (Utilities|IsValid _player)
          ;[1 1 1] Hit player
          (if (Variables|Default|GetIsSkillShot)
            (Class|NeedleDamageSystem|SkillShotHit (Actor|GetComponentbyClass _asbase_character "/Script/MoBArtFX.Needle_Damage_System") (Variables|Default|GetSlownessDelay) (Variables|Default|GetStunDelay))
            (elif (Variables|Default|GetIsTeleport)
              _
              (else
                (Class|NeedleDamageSystem|Hit (Actor|GetComponentbyClass _asbase_character "/Script/MoBArtFX.Needle_Damage_System") (Variables|Default|GetType) (Variables|Default|GetDamage)))))
          (Actor|DestroyActor))))
    (:CastFailed
      (if (!= OtherActor self)
        ;[1 1 1] Teleport player
        (if (Variables|Default|GetIsTeleport)
          (Transformation|SetActorLocation (Variables|Default|GetPlayer) (Transformation|GetActorLocation) false false)
          (Actor|DestroyActor)
          (else
            (Actor|DestroyActor)))))))

(fn ConstructionScript)