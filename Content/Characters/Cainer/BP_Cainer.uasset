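; BP_Cainer is the Blueprint for the playable character Cainer, adding a projectile auto attack and camera-shake feedback on top of parent logic.
; AutoAttack is cooldown-gated and, with ammo left, spawns a BP_CainerBullet given damage and bounce boost from CainerInfos.
; Tick counts the cooldown down, clearing the Shooting and Reloading flags meanwhile.
; Shooting, reloading, landing and MitigateDamage each play their own world camera shake.
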(event EventBeginPlay)

(event Collision|EventActorBeginOverlap
  (params (OtherActor :type Actor%20Object%20Reference)))

(event EventTick
  (params (DeltaSeconds :type Float%20%28single-precision%29))
  (if (> (Variables|Default|GetAutoAttackCD) 0.0)
    (Variables|Default|SetAutoAttackCD (- (Variables|Default|GetAutoAttackCD) DeltaSeconds))
    (Variables|Default|SetShooting false)
    (Variables|Default|SetReloading false)))

(event EventAutoAttack
  (bind _bulletstart (Variables|Default|GetBulletStart))
  (bind _returnvalue (Transformation|GetWorldRotation _bulletstart))
  (if (<= (Variables|Default|GetAutoAttackCD) 0.0)
    (if (> (Variables|/Script/MoBArtFX.PlayerInfos|GetCurrentAmmo (Class|BaseCharacter|GetPlayerDatas)) 0)
      (bind _returnvalue_2 (Game|SpawnActorfromClass "/Game/Characters/Cainer/Utils/BP_CainerBullet.BP_CainerBullet_C" (Math|Transform|MakeTransform (+ (Transformation|GetWorldLocation (Variables|Default|GetBulletStart)) _returnvalue) _returnvalue) "AlwaysSpawn" "MultiplyWithRoot" 0 0))
      (bind _ascainer_infos (Utilities|Casting|CastToCainerInfos (Class|BaseCharacter|GetPlayerDatas))
        (:then
          (Variables|/Game/Characters/Cainer/Utils/BP_CainerBullet.BP_CainerBullet_C|SetDamages _returnvalue_2 (Variables|/Script/MoBArtFX.CainerInfos|GetautoattackDamage _ascainer_infos))
          (Variables|/Game/Characters/Cainer/Utils/BP_CainerBullet.BP_CainerBullet_C|SetDamagePercentageBounceBoost _returnvalue_2 (Variables|/Script/MoBArtFX.CainerInfos|GetautoattackPercentageBounceBoost _ascainer_infos)))
        (:CastFailed
          _))
      (Camera|PlayWorldCameraShake "/Game/Characters/Cainer/CameraShakes/BP_ShootCShake.BP_ShootCShake_C" (Transformation|GetActorLocation) 0.0 5e+02)
      (Variables|Default|SetShooting true))
    (|CallParentFunction)
    (Variables|Default|SetAutoAttackCD (Variables|/Script/MoBArtFX.PlayerInfos|GetAutoAttack_CD (Class|BaseCharacter|GetPlayerDatas)))
    (else
      (Development|PrintString "Cainer's auto attack is on CD !" true true "(R=1.000000,G=0.000000,B=0.000000,A=1.000000)" 3.0))))

(event EventOnLanded
  (params (Hit :type Hit%20Result%20Structure%20%28by%20ref%29))
  (Camera|PlayWorldCameraShake "/Game/Characters/Cainer/CameraShakes/BP_JumpCShake.BP_JumpCShake_C" (Transformation|GetActorLocation) 0.0 5e+02))

(event EventReload
  (|CallParentFunction)
  (Camera|PlayWorldCameraShake "/Game/Characters/Cainer/CameraShakes/BP_ReloadCShake.BP_ReloadCShake_C" (Transformation|GetActorLocation) 0.0 5e+02)
  (Variables|Default|SetReloading true))

(fn ConstructionScript)

(fn MitigateDamage
  (params (damage :type Float%20%28single-precision%29) (causer :type Actor%20Object%20Reference))
  (bind _returnvalue (|CallParentFunction damage causer))
  (Camera|PlayWorldCameraShake "/Game/Characters/Cainer/CameraShakes/BP_DamageCShake.BP_DamageCShake_C" (Transformation|GetActorLocation) 0.0 5e+02)
  (return _returnvalue))