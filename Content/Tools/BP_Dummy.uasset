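; BP_Dummy is a test dummy that displays its current health and periodically fires at pawns in front of it.
; Each tick, a text render shows the health from its player data, tinted from red to green by the fraction of max health.
; A looping timer started at BeginPlay runs a debug-drawn forward sphere trace, applies damage to the hit actor and prints a debug string.
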(event Custom|Fire
  (bind _returnvalue (Transformation|GetActorLocation))
  (bind _outhit (Collision|SphereTraceForObjects _returnvalue (+ _returnvalue (* (Transformation|GetActorForwardVector) 1e+04)) 3e+01 (Utilities|Array|MakeArray "ObjectTypeQuery3") false 0 "ForDuration" true "(R=1.000000,G=0.000000,B=0.000000,A=1.000000)" "(R=0.000000,G=1.000000,B=0.000000,A=1.000000)" (- (Variables|Default|GetFireTime) 0.1)))
  (Game|Damage|ApplyDamage (.HitActor (Collision|BreakHitResult _outhit)) 1e+01 (Pawn|GetController) self)
  (Development|PrintString "Hello"))

(event EventBeginPlay
  (|CallParentFunction)
  (Utilities|Time|SetTimerbyEvent (delegate Custom|Fire) (Variables|Default|GetFireTime) true))

(event EventTick
  (params (DeltaSeconds :type Float%20%28single-precision%29))
  (bind _returnvalue (Class|BaseCharacter|GetPlayerDatas))
  (bind _textrender (Variables|Default|GetTextRender))
  (bind _currenthealth (Variables|/Script/MoBArtFX.PlayerInfos|GetCurrentHealth _returnvalue))
  (|CallParentFunction DeltaSeconds)
  (Rendering|Components|TextRender|SetText _textrender (Utilities|Text|ToText(Integer) _currenthealth))
  (Rendering|Components|TextRender|SetTextRenderColor _textrender (Math|Conversions|ToColor(LinearColor) (Math|Color|Lerp(LinearColor) "(R=1.000000,G=0.000000,B=0.000000,A=1.000000)" "(R=0.000000,G=1.000000,B=0.000000,A=1.000000)" (/ (Math|Conversions|ToFloat(Integer) _currenthealth) (Math|Conversions|ToFloat(Integer) (Variables|/Script/MoBArtFX.PlayerInfos|GetMaxHealth _returnvalue)))))))

(fn ConstructionScript
  (|CallParentFunction))