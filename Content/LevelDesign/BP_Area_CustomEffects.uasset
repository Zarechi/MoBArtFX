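; BP_Area_CustomEffects is a level-design area that spawns a Niagara effect when a BP_BaseCharacter enters its box.
; On overlap, it casts its DataAsset to PDA_Particles and spawns that asset's NiagaraEffects system at the character's location.
; Each overlap also replaces DataAsset with a new object constructed from the asset's class, so later overlaps read that instance rather than the originally assigned asset.
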(event OnComponentBeginOverlap(Box)
  (params (OverlappedComponent :type Primitive%20Component%20Object%20Reference) (OtherActor :type Actor%20Object%20Reference) (OtherComp :type Primitive%20Component%20Object%20Reference) (OtherBodyIndex :type Integer) (bFromSweep :type Boolean) (SweepResult :type Hit%20Result%20Structure%20%28by%20ref%29))
  (bind _asbp_base_character (Utilities|Casting|CastToBP_BaseCharacter OtherActor))
  ;[1 1 1] Instance Of Data Assets
  (bind _aspda_particles (Utilities|Casting|CastToPDA_Particles (Variables|Default|GetDataAsset)))
  (bind _returnvalue (Game|ConstructObjectfromClass (Utilities|GetClass _aspda_particles)))
  (Variables|Default|SetDataAsset _returnvalue)
  (Niagara|SpawnSystematLocation (Variables|/Game/LevelDesign/Data_Assets/PDA_Particles.PDA_Particles_C|GetNiagaraEffects _aspda_particles) (Transformation|GetActorLocation _asbp_base_character)))

(event EventBeginPlay
  (|CallParentFunction) ; This node is disabled and will not be called.\nDrag off pins to build functionality.
)

(event Collision|EventActorBeginOverlap
  (params (OtherActor :type Actor%20Object%20Reference))
  (|CallParentFunction OtherActor) ; This node is disabled and will not be called.\nDrag off pins to build functionality.
)

(event EventTick
  (params (DeltaSeconds :type Float%20%28single-precision%29))
  (|CallParentFunction DeltaSeconds) ; This node is disabled and will not be called.\nDrag off pins to build functionality.
)

(fn ConstructionScript
  (|CallParentFunction))