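; BPC_InkArea is a character component that shows an ink splash overlay on the player's screen and fades it out.
; On BeginPlay it async-loads the widget class from InkData and stretches the widget across the owning player's HUD viewport canvas.
; Tick stays off until StartFadeOut, then a normalized timer drives opacity through the InkData curve.
; When the timer completes, the component removes the widget and destroys itself.
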(event Custom|StartFadeOut
  (Components|Tick|SetComponentTickEnabled true)
  (Variables|Default|SetcurrentTimer 0.0))

(event Custom|SetupStartingValues
  (Components|Tick|SetComponentTickEnabled false)
  (Widget|SetRenderOpacity (Variables|Default|GetWidgetRef) 1.0))

(event EventBeginPlay
  ;[0.069 0.05115 0.2135] Create Widget
  (bind _class (Utilities|AsyncLoadClassAsset (.inksplashwidget (Variables|Default|GetInkData)))
    (:Completed
      (bind _asuser_widget (Utilities|Casting|CastToUserWidgetClass _class))
      (bind _returnvalue (UserInterface|CreateWidget _asuser_widget))
      (Variables|Default|SetWidgetRef _returnvalue)
      ;[0.1927 0.07662 0.04178] Get the Player's local viewport
      (bind _output_get (Variables|Default|SetOwner (Components|GetOwner)))
      (bind _asbase_character (Utilities|Casting|CastToBaseCharacter _output_get))
      (bind _asplayer_controller (Utilities|Casting|CastToPlayerController (Pawn|GetController _asbase_character)))
      (bind _ashud_mo_bart_fx (Utilities|Casting|CastToHUD_MoBArtFX (HUD|GetHUD _asplayer_controller)))
      ;[0.009641 0.05208 0.01139] Add the widget and set it up
      (bind _returnvalue_2 (Class|CanvasPanel|AddChildtoCanvas (Variables|/Game/_GameManager/UI/WBP_ViewportBase.WBP_ViewportBase_C|GetCanvasBase (.AsWBP%20Viewport%20Base (Utilities|Casting|CastToWBP_ViewportBase (Variables|/Script/MoBArtFX.HUD_MoBArtFX|GetViewportInstance _ashud_mo_bart_fx)))) (Variables|Default|GetWidgetRef)))
      (Class|CanvasPanelSlot|SetAnchors _returnvalue_2 (Utilities|Struct|MakeAnchors "(X=0.000000,Y=0.000000)" "(X=1.000000,Y=1.000000)"))
      (Class|CanvasPanelSlot|SetOffsets _returnvalue_2)
      (CallFunction|SetupStartingValues))))

(event EventTick
  (params (DeltaSeconds :type Float%20%28single-precision%29))
  (CallFunction|IncreaseFadeOutTimer))

(fn IncreaseFadeOutTimer
  (bind _return (CallFunction|IncreaseValueFloat (Variables|Default|GetcurrentTimer) (/ (Utilities|Time|GetWorldDeltaSeconds) (.fadeoutduration (Variables|Default|GetInkData)))))
  (if (>= _return 1.0)
    ;[0.1094 0.02988 0.06605] Destroy Widget & Self
    (Widget|RemovefromParent (Variables|Default|GetWidgetRef))
    (Components|DestroyComponent)
    (else
      (bind _widgetref (Variables|Default|GetWidgetRef)
        (:then
          (Widget|SetRenderOpacity _widgetref (Math|Curves|GetFloatValue (.fadeoutcurve (Variables|Default|GetInkData)) (Variables|Default|GetcurrentTimer))))
        (:else)))))