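; Radioactive area actor that tints the BP_TurboMaurice4000 camera while it is inside.
; On overlap it saves the camera's saturation and intensity, then opens a gate so Tick interpolates both toward BaseDataArea values.
; On Box exit it closes that gate; interpolation back to the saved values is wired to this one-off event, not Tick.
; The cast to PDA_PrimairDataasset in this graph never runs.
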(event OnComponentEndOverlap(Box)
  (params (OverlappedComponent :type Primitive%20Component%20Object%20Reference) (OtherActor :type Actor%20Object%20Reference) (OtherComp :type Primitive%20Component%20Object%20Reference) (OtherBodyIndex :type Integer))
  (bind _returnvalue (Utilities|Time|GetWorldDeltaSeconds))
  (bind _returnvalue_2 (Utilities|Time|GetWorldDeltaSeconds))
  (bind _basedataarea (Variables|Default|GetBaseDataArea))
  (bind _saturation (Variables|Default|GetSaturation))
  (bind (_x _y _z _w) (Math|Vector4|BreakVector4 _saturation))
  (bind _effectcolor (Variables|/Game/LevelDesign/Data_Radioactif/PDA_PrimairDataasset.PDA_PrimairDataasset_C|GetEffectColor _basedataarea))
  (bind _saturation_2 (Utilities|Struct|BreakColorGradePerRangeSettings _effectcolor))
  (bind (_x_2 _y_2 _z_2 _w_2) (Math|Vector4|BreakVector4 _saturation_2))
  (bind _asbp_turbo_maurice_4000 (Utilities|Casting|CastToBP_TurboMaurice4000 OtherActor))
  (Utilities|FlowControl|Sequence
    (:then_0
      (Utilities|FlowControl|Gate true) ; enters at Close
    )
    (:then_1
      (Utilities|FlowControl|Gate true
        (:Exit
          (Variables|/Script/Engine.CameraComponent|SetPostProcessSettings (Variables|/Game/Characters/TurboMaurice4000/BP_TurboMaurice4000.BP_TurboMaurice4000_C|GetCamera _asbp_turbo_maurice_4000) (Utilities|Struct|MakePostProcessSettings (Math|Vector4|MakeVector4 (Math|Interpolation|FInterpTo (.X (Math|Vector4|BreakVector4 (.ColorSaturation (Utilities|Struct|BreakPostProcessSettings (Variables|/Script/Engine.CameraComponent|GetPostProcessSettings (Variables|/Game/Characters/TurboMaurice4000/BP_TurboMaurice4000.BP_TurboMaurice4000_C|GetCamera _asbp_turbo_maurice_4000)))))) _x _returnvalue 4.0) (Math|Interpolation|FInterpTo (.Y (Math|Vector4|BreakVector4 (.ColorSaturation (Utilities|Struct|BreakPostProcessSettings (Variables|/Script/Engine.CameraComponent|GetPostProcessSettings (Variables|/Game/Characters/TurboMaurice4000/BP_TurboMaurice4000.BP_TurboMaurice4000_C|GetCamera _asbp_turbo_maurice_4000)))))) _y _returnvalue 4.0) (Math|Interpolation|FInterpTo (.Z (Math|Vector4|BreakVector4 (.ColorSaturation (Utilities|Struct|BreakPostProcessSettings (Variables|/Script/Engine.CameraComponent|GetPostProcessSettings (Variables|/Game/Characters/TurboMaurice4000/BP_TurboMaurice4000.BP_TurboMaurice4000_C|GetCamera _asbp_turbo_maurice_4000)))))) _z _returnvalue 4.0) (Math|Interpolation|FInterpTo (.W (Math|Vector4|BreakVector4 (.ColorSaturation (Utilities|Struct|BreakPostProcessSettings (Variables|/Script/Engine.CameraComponent|GetPostProcessSettings (Variables|/Game/Characters/TurboMaurice4000/BP_TurboMaurice4000.BP_TurboMaurice4000_C|GetCamera _asbp_turbo_maurice_4000)))))) _w _returnvalue 4.0)) (Math|Interpolation|FInterpTo (.SceneFringeIntensity (Utilities|Struct|BreakPostProcessSettings (Variables|/Script/Engine.CameraComponent|GetPostProcessSettings (Variables|/Game/Characters/TurboMaurice4000/BP_TurboMaurice4000.BP_TurboMaurice4000_C|GetCamera _asbp_turbo_maurice_4000)))) (Variables|Default|GetIntensity) _returnvalue 4.0))))))))

(event EventBeginPlay
  (|CallParentFunction))

(event Collision|EventActorBeginOverlap
  (params (OtherActor :type Actor%20Object%20Reference))
  (bind _returnvalue (Utilities|Time|GetWorldDeltaSeconds))
  (bind _basedataarea (Variables|Default|GetBaseDataArea))
  (bind _effectcolor (Variables|/Game/LevelDesign/Data_Radioactif/PDA_PrimairDataasset.PDA_PrimairDataasset_C|GetEffectColor _basedataarea))
  (bind _saturation (Utilities|Struct|BreakColorGradePerRangeSettings _effectcolor))
  (bind (_x _y _z _w) (Math|Vector4|BreakVector4 _saturation))
  ;[1 1 1] Comment
  (|CallParentFunction OtherActor)
  (bind _asbp_turbo_maurice_4000 (Utilities|Casting|CastToBP_TurboMaurice4000 OtherActor))
  (Variables|Default|SetIntensity (.SceneFringeIntensity (Utilities|Struct|BreakPostProcessSettings (Variables|/Script/Engine.CameraComponent|GetPostProcessSettings (Variables|/Game/Characters/TurboMaurice4000/BP_TurboMaurice4000.BP_TurboMaurice4000_C|GetCamera _asbp_turbo_maurice_4000)))))
  (Variables|Default|SetSaturation (.ColorSaturation (Utilities|Struct|BreakPostProcessSettings (Variables|/Script/Engine.CameraComponent|GetPostProcessSettings (Variables|/Game/Characters/TurboMaurice4000/BP_TurboMaurice4000.BP_TurboMaurice4000_C|GetCamera _asbp_turbo_maurice_4000)))))
  (Utilities|FlowControl|Gate true) ; enters at Open
)

(event EventTick
  (params (DeltaSeconds :type Float%20%28single-precision%29))
  (bind _returnvalue (Utilities|Time|GetWorldDeltaSeconds))
  (bind _basedataarea (Variables|Default|GetBaseDataArea))
  (bind _effectcolor (Variables|/Game/LevelDesign/Data_Radioactif/PDA_PrimairDataasset.PDA_PrimairDataasset_C|GetEffectColor _basedataarea))
  (bind _saturation (Utilities|Struct|BreakColorGradePerRangeSettings _effectcolor))
  (bind (_x _y _z _w) (Math|Vector4|BreakVector4 _saturation))
  (|CallParentFunction DeltaSeconds)
  (Utilities|FlowControl|Gate true
    (:Exit
      (Variables|/Script/Engine.CameraComponent|SetPostProcessSettings (Variables|/Game/Characters/TurboMaurice4000/BP_TurboMaurice4000.BP_TurboMaurice4000_C|GetCamera (stale Collision|EventActorBeginOverlap _asbp_turbo_maurice_4000)) (Utilities|Struct|MakePostProcessSettings (Math|Vector4|MakeVector4 (Math|Interpolation|FInterpTo (.X (Math|Vector4|BreakVector4 (.ColorSaturation (Utilities|Struct|BreakPostProcessSettings (Variables|/Script/Engine.CameraComponent|GetPostProcessSettings (Variables|/Game/Characters/TurboMaurice4000/BP_TurboMaurice4000.BP_TurboMaurice4000_C|GetCamera (stale Collision|EventActorBeginOverlap _asbp_turbo_maurice_4000))))))) _x _returnvalue 4.0) (Math|Interpolation|FInterpTo (.Y (Math|Vector4|BreakVector4 (.ColorSaturation (Utilities|Struct|BreakPostProcessSettings (Variables|/Script/Engine.CameraComponent|GetPostProcessSettings (Variables|/Game/Characters/TurboMaurice4000/BP_TurboMaurice4000.BP_TurboMaurice4000_C|GetCamera (stale Collision|EventActorBeginOverlap _asbp_turbo_maurice_4000))))))) _y _returnvalue 4.0) (Math|Interpolation|FInterpTo (.Z (Math|Vector4|BreakVector4 (.ColorSaturation (Utilities|Struct|BreakPostProcessSettings (Variables|/Script/Engine.CameraComponent|GetPostProcessSettings (Variables|/Game/Characters/TurboMaurice4000/BP_TurboMaurice4000.BP_TurboMaurice4000_C|GetCamera (stale Collision|EventActorBeginOverlap _asbp_turbo_maurice_4000))))))) _z _returnvalue 4.0) (Math|Interpolation|FInterpTo (.W (Math|Vector4|BreakVector4 (.ColorSaturation (Utilities|Struct|BreakPostProcessSettings (Variables|/Script/Engine.CameraComponent|GetPostProcessSettings (Variables|/Game/Characters/TurboMaurice4000/BP_TurboMaurice4000.BP_TurboMaurice4000_C|GetCamera (stale Collision|EventActorBeginOverlap _asbp_turbo_maurice_4000))))))) _w _returnvalue 4.0)) (Math|Interpolation|FInterpTo (.SceneFringeIntensity (Utilities|Struct|BreakPostProcessSettings (Variables|/Script/Engine.CameraComponent|GetPostProcessSettings (Variables|/Game/Characters/TurboMaurice4000/BP_TurboMaurice4000.BP_TurboMaurice4000_C|GetCamera (stale Collision|EventActorBeginOverlap _asbp_turbo_maurice_4000))))) (Variables|/Game/LevelDesign/Data_Radioactif/PDA_PrimairDataasset.PDA_PrimairDataasset_C|GetIntensity _basedataarea) _returnvalue 4.0))))))

(fn ConstructionScript
  (|CallParentFunction))