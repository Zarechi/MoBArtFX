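; Boost component that rewrites the player character's current health a single time, when play begins.
; BeginPlay casts player 0's character to BP_BaseCharacter and sets CurrentHealth in its player data to (health + 10) scaled by a fifth of the frame delta, truncated to a whole number.
; Because of that scaling, the result is normally near zero rather than a heal; Tick is empty, so nothing repeats.
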(event EventBeginPlay
  (bind _asbp_base_character (Utilities|Casting|CastToBP_BaseCharacter (Game|GetPlayerCharacter 0)))
  (Variables|/Script/MoBArtFX.PlayerInfos|SetCurrentHealth (Class|BaseCharacter|GetPlayerDatas _asbp_base_character) (Math|Conversions|ToFloat(Integer) (Math|Float|Truncate (* (+ (Variables|/Script/MoBArtFX.PlayerInfos|GetCurrentHealth (Class|BaseCharacter|GetPlayerDatas _asbp_base_character)) 10) (/ (Utilities|Time|GetWorldDeltaSeconds) 5.0))))))

(event EventTick
  (params (DeltaSeconds :type Float%20%28single-precision%29)))