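; BP_AreaGustav is a trigger area that runs a data asset's message on the player and plays a camera FOV effect.
; When BP_Player_Gustav overlaps it, a Timeline widens the first-person camera FOV, then reverses after a short delay.
; The PrimaryDataAsset executes its DatasMessage on the character shortly after overlap.
; BeginPlay also builds an instance copy of that asset's message, though the overlap uses the original asset.
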(event EventBeginPlay
  (bind _primarydataasset (Variables|Default|GetPrimaryDataAsset)
    (:then
      (bind _returnvalue (Game|ConstructObjectfromClass (Utilities|GetClass _primarydataasset)))
      (Variables|Default|SetDataAsset_Inst _returnvalue)
      (bind _datastruct (Class|BPILDAreaGustav|GetDatas(Message) (Variables|Default|GetPrimaryDataAsset)))
      (Class|BPILDAreaGustav|SetDatas(Message) (Variables|Default|GetDataAsset_Inst) _datastruct))
    (:else)))

(event Collision|EventActorBeginOverlap
  (params (OtherActor :type Actor%20Object%20Reference))
  (bind _ascharacter (Utilities|Casting|CastToCharacter OtherActor))
  (bind _asbp_player_gustav (Utilities|Casting|CastToBP_Player_Gustav _ascharacter))
  (Utilities|FlowControl|Sequence
    (:then_0
      (Utilities|FlowControl|Delay 0.2)
      (Class|BPILDAreaGustav|ExecuteDatas(Message) (Variables|Default|GetPrimaryDataAsset) _ascharacter))
    (:then_1
      (bind _fov (Timeline|Timeline PlayFromStart)
        (:Update
          (Variables|/Script/Engine.CameraComponent|SetFieldOfView (Variables|/Game/GustavTeam/Gustav/Character/BP_Player_Gustav.BP_Player_Gustav_C|GetFirstPersonCamera _asbp_player_gustav) (Math|Float|Lerp 125.0 175.0 _fov)))))
    (:then_2
      (Utilities|FlowControl|Delay 0.4)
      (Timeline|Timeline ReverseFromEnd))))

(fn ConstructionScript)