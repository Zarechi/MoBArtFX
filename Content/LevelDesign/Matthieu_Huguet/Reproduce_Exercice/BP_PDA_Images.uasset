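; BP_PDA_Images is a data Blueprint that holds a structure whose Images field supplies a material for Change_Color_Box actors.
; CopyData writes its structure into another BP_PDA_Images asset.
; ExecuteReference casts the given actor to Change_Color_Box and applies that material to slot 0 of its static mesh.
; Both events do nothing when their cast fails, and SetData is an empty function.
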(event EventCopyData
  (params (ToAsset :type Primary%20Data%20Asset%20Object%20Reference%20%28by%20ref%29))
  (bind _asbp_pda_images (Utilities|Casting|CastToBP_PDA_Images ToAsset))
  (Variables|BP_PDA_Images_C|SetStructure _asbp_pda_images (Variables|Default|GetStructure)))

(event EventExecuteReference
  (params (Actor :type Actor%20Object%20Reference))
  (bind _asbox_actor (Utilities|Casting|CastToChange_Color_Box Actor))
  (Rendering|Material|SetMaterial (Variables|/Game/LevelDesign/Matthieu_Huguet/Change_Color_Box.Change_Color_Box_C|GetStaticMesh _asbox_actor) 0 (Utilities|Struct|BreakF_Struct_Images (Variables|Default|GetStructure))))

(fn SetData
  (return ""))