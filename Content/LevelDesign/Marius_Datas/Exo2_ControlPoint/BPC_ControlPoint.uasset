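; BPC_ControlPoint is a control point component, in an exercise folder, that eases a test value toward 100 over time.
; StartValue enables ticking, and each tick calls Test, which advances Supertest with FInterpTo and prints it for debugging.
; ResetStartingValue only disables ticking, so the value pauses where it is instead of resetting.
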(event Custom|Test
  (bind _output_get (Variables|Default|SetSupertest (Math|Interpolation|FInterpTo (Variables|Default|GetSupertest) 1e+02 (Utilities|Time|GetWorldDeltaSeconds) 1.0)))
  (Development|PrintString (Utilities|String|ToString(Float) _output_get)))

(event Custom|ResetStartingValue
  (Components|Tick|SetComponentTickEnabled false))

(event Custom|StartValue
  (Components|Tick|SetComponentTickEnabled true))

(event EventBeginPlay)

(event EventTick
  (params (DeltaSeconds :type Float%20%28single-precision%29))
  (CallFunction|Test))